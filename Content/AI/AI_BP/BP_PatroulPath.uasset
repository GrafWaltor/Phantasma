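; BP_PatroulPath is a patrol route for AI, defined by the spline component PatroulRout.
; IncrementPatrolPath steps PatroulIndex along the spline points, flipping Direction at the last and first points so the route runs back and forth.
; GetSplinePointsInWorldPosition returns the world location of the spline point at the current index.
; The index and direction are stored on the path itself.
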(event Custom|IncrementPatrolPath
  (bind _output_get (Variables|Default|SetPatroulIndex (+ (Variables|Default|GetPatroulIndex) (Variables|Default|GetDirection))))
  (if (== _output_get (- (Spline|GetNumberOfSplinePoints (Variables|Default|GetPatroulRout)) 1))
    (Variables|Default|SetDirection -1)
    (elif (== (Variables|Default|GetPatroulIndex) 0)
      (Variables|Default|SetDirection 1))))

(fn ConstructionScript)

(fn GetSplinePointsinWorldPosition
  (return (Spline|GetLocationatSplinePoint (Variables|Default|GetPatroulRout) (Variables|Default|GetPatroulIndex) "World")))