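; BP_Camera is a follow camera actor that tracks FollowTarget in the XZ plane while keeping its own Y position, as in a side-on view.
; Every Tick, UpdateCamera offsets the target's location along its forward vector by CamOffset, using only X and Z, so the camera leads toward the target's facing.
; The actor eases to that point with VInterpTo at InterpSpeed, without sweeping.
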(event EventBeginPlay)

(event Collision|EventActorBeginOverlap
  (params (OtherActor :type Actor%20Object%20Reference)))

(event EventTick
  (params (DeltaSeconds :type Float%20%28single-precision%29))
  (CallFunction|UpdateCamera))

(fn ConstructionScript)

(fn UpdateCamera
  (bind _returnvalue (Transformation|GetActorLocation))
  (bind _followtarget (Variables|Default|GetFollowTarget))
  (bind _followtarget_2 (Variables|Default|GetFollowTarget))
  (bind _camoffset (Variables|Default|GetCamOffset))
  (bind _returnvalue_2 (Transformation|GetActorForwardVector _followtarget_2))
  (bind _returnvalue_3 (Transformation|GetActorLocation _followtarget))
  (bind _returnvalue_4 (* _returnvalue_2 _camoffset))
  (Transformation|SetActorLocation (Math|Interpolation|VInterpTo (Math|Vector|MakeVector (.x _returnvalue) (.y _returnvalue) (.z _returnvalue)) (+ (Math|Vector|MakeVector (.x _returnvalue_3) (.y (Transformation|GetActorLocation)) (.z _returnvalue_3)) (Math|Vector|MakeVector (.x _returnvalue_4) 0.0 (.z _returnvalue_4))) (Utilities|Time|GetWorldDeltaSeconds) (Variables|Default|GetInterp%20Speed)) false false))