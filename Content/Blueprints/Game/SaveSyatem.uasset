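; SaveSyatem is a checkpoint-style actor that records a respawn point in BP_GameMode.
; Any overlap of its Box sets OpenRespawn and stores the sweep result's location as RespLocation, with no check on the overlapping actor.
; A Death event destroys this actor, and its Destroyed event calls the game mode's Respawn.
; A Russian note marks the Death logic for moving into the character.
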(event OnComponentBeginOverlap(Box)
  (params (OverlappedComponent :type Primitive%20Component%20Object%20Reference) (OtherActor :type Actor%20Object%20Reference) (OtherComp :type Primitive%20Component%20Object%20Reference) (OtherBodyIndex :type Integer) (bFromSweep :type Boolean) (SweepResult :type Hit%20Result%20Structure%20%28by%20ref%29))
  (Variables|Default|SetOpenRespawn true)
  (Variables|Default|Setlocation (Math|Conversions|ToTransform(Vector) (.Location (Collision|BreakHitResult SweepResult))))
  (bind _asbp_game_mode (Utilities|Casting|CastToBP_GameMode (Game|GetGameMode)))
  (Variables|/Game/Blueprints/Game/BP_GameMode.BP_GameMode_C|SetRespLocation _asbp_game_mode (Variables|Default|Getlocation)))

(event Custom|Death
  ;[1 1 1] перенести в чара
  (Actor|DestroyActor))

(event EventBeginPlay)

(event EventTick
  (params (DeltaSeconds :type Float%20%28single-precision%29)))

(event Collision|EventActorBeginOverlap
  (params (OtherActor :type Actor%20Object%20Reference)))

(event EventDestroyed
  ;[1 1 1] перенести в чара
  (bind _asbp_game_mode (Utilities|Casting|CastToBP_GameMode (Game|GetGameMode)))
  (Default|Respawn _asbp_game_mode))

(fn ConstructionScript)