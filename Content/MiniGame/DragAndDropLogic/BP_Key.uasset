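; BP_Key is a key actor that the player drags with the mouse in a drag-and-drop minigame.
; BeginPlay enables the cursor and click events and adds a physics handle to the player controller.
; Clicking the key mesh grabs the component under a Visibility trace, and releasing drops it.
; While dragging, Tick moves the handle target to a separate-channel cursor trace's X/Y at zero height, printing the hit component's name.
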(event OnClicked(SM_Key)
  (params (TouchedComponent :type Primitive%20Component%20Object%20Reference) (ButtonPressed :type Key%20Structure :default "None"))
  (bind _playercontrollerref (Variables|Components|GetPlayerControllerRef))
  (bind _hitresult (Game|Player|GetHitResultUnderCursorbyChannel _playercontrollerref "TraceTypeQuery1" false))
  (bind (_bblockinghit _binitialoverlap _time _distance _location _impactpoint _normal _impactnormal _physmat _hitactor _hitcomponent) (Collision|BreakHitResult _hitresult))
  (if _bblockinghit
    (Class|PhysicsHandleComponent|GrabComponentatLocation (Variables|Default|GetPhysicsHandle) _hitcomponent "None" (Transformation|GetWorldLocation _hitcomponent))
    (Variables|Components|SetbIsDragging true)))

(event OnReleased(SM_Key)
  (params (TouchedComponent :type Primitive%20Component%20Object%20Reference) (ButtonReleased :type Key%20Structure :default "None"))
  (Physics|Components|PhysicsHandle|ReleaseComponent (Variables|Default|GetPhysicsHandle))
  (Variables|Components|SetbIsDragging false))

(event EventBeginPlay
  (bind _output_get (Variables|Components|SetPlayerControllerRef (Game|GetPlayerController 0)))
  (Variables|/Script/Engine.PlayerController|SetbShowMouseCursor _output_get true)
  (Variables|/Script/Engine.PlayerController|SetbEnableClickEvents _output_get true)
  (bind _returnvalue (AddComponent|AddPhysicsHandleComponent _output_get))
  (Variables|Default|SetPhysicsHandle _returnvalue))

(event EventTick
  (params (DeltaSeconds :type Float%20%28single-precision%29))
  (bind _playercontrollerref (Variables|Components|GetPlayerControllerRef))
  (bind _hitresult (Game|Player|GetHitResultUnderCursorbyChannel _playercontrollerref "TraceTypeQuery5" false))
  (bind (_bblockinghit _binitialoverlap _time _distance _location _impactpoint _normal _impactnormal _physmat _hitactor _hitcomponent) (Collision|BreakHitResult _hitresult))
  (if (Variables|Components|GetbIsDragging)
    (Physics|Components|PhysicsHandle|SetTargetLocation (Variables|Default|GetPhysicsHandle) (Math|Vector|MakeVector (.x _location) (.y _location) 0.0))
    (Development|PrintString (Utilities|GetDisplayName _hitcomponent))))

(fn ConstructionScript)