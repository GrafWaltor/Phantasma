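; BP_KeyPawn_1 is a controllable pawn for a pawn-switching minigame, with its static mesh hidden at start.
; On possession it adds the default Enhanced Input mapping and caches the third-person character.
; Input drives planar movement relative to control rotation and vertical movement along actor up, both scaled through FInterpTo, plus local yaw rotation.
; SwitchToCharacter repossesses the cached character and sets the view target to BP_Camera.
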(event Input|EnhancedActionEvents|EnhancedInputActionIA_Move
  (params (ActionValue :type Vector :default "0, 0, 0") (ElapsedSeconds :type Float%20%28double-precision%29) (TriggeredSeconds :type Float%20%28double-precision%29) (InputAction :type Input%20Action%20Object%20Reference :default "/Game/ThirdPerson/Input/Actions/IA_Move.IA_Move"))
  (bind _returnvalue (Pawn|GetControlRotation :!class /Script/Engine.Pawn))
  (bind _returnvalue_2 (Pawn|GetControlRotation :!class /Script/Engine.Pawn))
  (Pawn|Input|AddMovementInput (Math|Vector|GetRightVector (Math|Rotator|MakeRotator (.roll _returnvalue_2) (.pitch _returnvalue_2) (.yaw _returnvalue_2))) (Math|Interpolation|FInterpTo (Variables|Default|GetCurrentValue) (.y ActionValue) (Utilities|Time|GetWorldDeltaSeconds) 1e+01) false)
  (Pawn|Input|AddMovementInput (* (Math|Vector|GetForwardVector (Math|Rotator|MakeRotator (.roll _returnvalue) (.pitch _returnvalue) (.yaw _returnvalue))) "-1.000000,-1.000000,-1.000000") (Math|Interpolation|FInterpTo (Variables|Default|GetCurrentValue) (.x ActionValue) (Utilities|Time|GetWorldDeltaSeconds) 1e+01) false))

(event Input|EnhancedActionEvents|EnhancedInputActionIA_PawnMove_UD
  (params (ActionValue :type Vector :default "0, 0, 0") (ElapsedSeconds :type Float%20%28double-precision%29) (TriggeredSeconds :type Float%20%28double-precision%29) (InputAction :type Input%20Action%20Object%20Reference :default "/Game/ThirdPerson/Input/Actions/IA_PawnMove_UD.IA_PawnMove_UD"))
  (Pawn|Input|AddMovementInput (Transformation|GetActorUpVector) (Math|Interpolation|FInterpTo (Variables|Default|GetCurrentValue) (.x ActionValue) (Utilities|Time|GetWorldDeltaSeconds) 1e+01) false))

(event Input|EnhancedActionEvents|EnhancedInputActionIA_RotatePawn
  (params (ActionValue :type Vector :default "0, 0, 0") (ElapsedSeconds :type Float%20%28double-precision%29) (TriggeredSeconds :type Float%20%28double-precision%29) (InputAction :type Input%20Action%20Object%20Reference :default "/Game/ThirdPerson/Input/Actions/IA_RotatePawn.IA_RotatePawn"))
  (Transformation|AddActorLocalRotation (Math|Rotator|MakeRotator 0.0 0.0 (* (.x ActionValue) (Variables|Default|GetRotationSpeed))) false false))

(event EventBeginPlay
  (Rendering|SetVisibility (Variables|Default|GetStaticMesh) false false))

(event EventPossessed
  (params (NewController :type Controller%20Object%20Reference))
  (bind _asplayer_controller (Utilities|Casting|CastToPlayerController (Pawn|GetController)))
  (bind _output_get (Variables|Default|SetAs%20Player%20Controller _asplayer_controller))
  (Utilities|IsValid _output_get
    (:Is%20Valid
      (Input|AddMappingContext (PlayerController|LocalPlayerSubsystems|GetEnhancedInputLocalPlayerSubsystem _asplayer_controller) "/Game/ThirdPerson/Input/IMC_Default.IMC_Default" 0 "(bIgnoreAllPressedKeysUntilRelease=True,bForceImmediately=False,bNotifyUserSettings=False)")
      (bind _returnvalue (Actor|GetActorOfClass "/Game/ThirdPerson/Blueprints/BP_ThirdPersonCharacter.BP_ThirdPersonCharacter_C"))
      (Variables|Default|SetPlayerCharacterRef _returnvalue))))

(fn ConstructionScript)

(fn SwitchtoCharacter
  (Pawn|Possess (Game|GetPlayerController 0) (Variables|Default|GetPlayerCharacterRef))
  (bind _returnvalue (Actor|GetActorOfClass "/Game/Blueprints/Game/BP_Camera.BP_Camera_C"))
  (bind _output_get (Variables|Default|SetDefaultCameraREF _returnvalue))
  (Game|Player|SetViewTargetwithBlend (Variables|Default|GetAs%20Player%20Controller) _output_get 0.0 "VTBlend_Linear" 0.0 false))