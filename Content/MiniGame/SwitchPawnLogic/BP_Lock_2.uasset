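; BP_Lock_2 is the lock in the second key minigame, started when something overlaps its StartGameBox.
; The overlap switches the player to the minigame, reveals BP_KeyPawn_2's mesh and loops a timer that triggers audio and a HUD hit animation.
; Key transform events run Compare, matching arrow X/Y and normalized yaw within tolerance.
; A match outlines the lock, returns control to the character, clears widgets and destroys both key and lock.
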(event OnComponentBeginOverlap(StartGameBox)
  (params (OverlappedComponent :type Primitive%20Component%20Object%20Reference) (OtherActor :type Actor%20Object%20Reference) (OtherComp :type Primitive%20Component%20Object%20Reference) (OtherBodyIndex :type Integer) (bFromSweep :type Boolean) (SweepResult :type Hit%20Result%20Structure%20%28by%20ref%29))
  (bind _playercharacterref (Variables|Default|GetPlayerCharacterREF))
  (Default|SwitchtoMiniGame2 _playercharacterref)
  (Rendering|SetActorHiddenInGame _playercharacterref true)
  (Rendering|SetVisibility (Variables|/Game/MiniGame/SwitchPawnLogic/BP_KeyPawn_2.BP_KeyPawn_2_C|GetStaticMesh (Variables|Default|GetKeyPawnRef)) true false)
  (Utilities|Time|SetTimerbyEvent (delegate Custom|AudioCriss) 5.0 true))

(event Custom|KeyTransformEvent
  (bind _keypawnref (Variables|Default|GetKeyPawnRef))
  (bind _match (CallFunction|Compare))
  (if _match
    (Input|DisableInput _keypawnref 0)
    (Rendering|Material|SetOverlayMaterial (Variables|Default|GetStaticMesh) "/Game/Phantasma/Materials/MI_OverlayOutline.MI_OverlayOutline" :!class /Script/Engine.MeshComponent)
    (Rendering|SetVisibility (Variables|/Game/MiniGame/SwitchPawnLogic/BP_KeyPawn_2.BP_KeyPawn_2_C|GetStaticMesh _keypawnref) false false)
    (Utilities|FlowControl|Delay 1.0)
    (Default|SwitchtoCharacter _keypawnref)
    (Viewport|RemoveAllWidgets)
    (Rendering|SetActorHiddenInGame (Variables|Default|GetPlayerCharacterREF) false)
    (Actor|DestroyActor _keypawnref)
    (Actor|DestroyActor)))

(event Custom|AudioCriss
  (Components|Activation|Activate (Variables|Default|GetAudio) false)
  (CallFunction|StartMindBreakerTimer))

(event EventBeginPlay
  (bind _returnvalue (Actor|GetActorOfClass "/Game/Phantasma/Blueprints/BP_Player_Game.BP_Player_Game_C"))
  (bind _output_get (Variables|Default|SetPlayerCharacterREF _returnvalue))
  (Utilities|IsValid _output_get
    (:Is%20Valid
      (bind _returnvalue_2 (Actor|GetActorOfClass "/Game/MiniGame/SwitchPawnLogic/BP_KeyPawn_2.BP_KeyPawn_2_C"))
      (bind _output_get_2 (Variables|Default|SetKeyPawnRef _returnvalue_2))
      (EventDispatchers|BindEventtoOnKeyTransform _output_get_2 (delegate Custom|KeyTransformEvent)))))

(fn ConstructionScript)

(fn NormalizeAngle
  (params (Agnle :type Float%20%28double-precision%29))
  (bind _returnvalue (Math|Rotator|NormalizeAxis Agnle))
  (return (Math|Float|SelectFloat _returnvalue (+ _returnvalue 3.6e+02) (>= _returnvalue 0.0))))

(fn Compare
  (bind _arrow (Variables|Default|GetArrow))
  (bind _keypawnref (Variables|Default|GetKeyPawnRef))
  (bind _returnvalue (Transformation|GetWorldLocation _arrow))
  (bind _keyarrow (Variables|/Game/MiniGame/SwitchPawnLogic/BP_KeyPawn_2.BP_KeyPawn_2_C|GetKeyArrow _keypawnref))
  (bind _returnvalue_2 (Transformation|GetWorldLocation _keyarrow))
  (if (and (Math|Float|NearlyEqual(Float) (.x _returnvalue) (.x _returnvalue_2) 5.0) (Math|Float|NearlyEqual(Float) (.y _returnvalue) (.y _returnvalue_2) 5.0))
    (bind _newangle (CallFunction|NormalizeAngle (.yaw (Transformation|GetWorldRotation (Variables|Default|GetArrow)))))
    (bind _newangle_2 (CallFunction|NormalizeAngle (.yaw (Transformation|GetWorldRotation _keyarrow))))
    (return (Math|Float|NearlyEqual(Float) _newangle _newangle_2 5.0))))

(fn StartMindBreakerTimer
  (bind _returnvalue (UserInterface|CreateWidget "/Game/Phantasma/UMG/Player/UI_Player_HUD1.UI_Player_HUD1_C" (Game|GetPlayerController 0)))
  (UserInterface|Viewport|AddtoViewport _returnvalue 0)
  (Default|PlayUIPillowHitAnimation _returnvalue)
  (Utilities|Time|SetTimerbyEvent (EventDispatchers|CreateEvent :!event ResetKeyLocation) 3.0))

(fn ResetKeyLocation)