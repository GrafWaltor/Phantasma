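; BP_Lock_1 is a lock actor that starts and ends a key-pawn minigame.
; On BeginPlay it caches the third-person character and, if that is valid, BP_KeyPawn_1.
; StartGameBox overlap calls SwitchPawnToMiniGame2 on the character and shows the key's mesh.
; OverlapBox overlap calls SwitchToCharacter on the key pawn, then destroys both key and lock, without filtering the overlapping actor.
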(event OnComponentBeginOverlap(OverlapBox)
  (params (OverlappedComponent :type Primitive%20Component%20Object%20Reference) (OtherActor :type Actor%20Object%20Reference) (OtherComp :type Primitive%20Component%20Object%20Reference) (OtherBodyIndex :type Integer) (bFromSweep :type Boolean) (SweepResult :type Hit%20Result%20Structure%20%28by%20ref%29))
  (bind _keypawnref (Variables|Default|GetKeyPawnRef))
  (Default|SwitchtoCharacter _keypawnref)
  (Actor|DestroyActor _keypawnref)
  (Actor|DestroyActor))

(event OnComponentBeginOverlap(StartGameBox)
  (params (OverlappedComponent :type Primitive%20Component%20Object%20Reference) (OtherActor :type Actor%20Object%20Reference) (OtherComp :type Primitive%20Component%20Object%20Reference) (OtherBodyIndex :type Integer) (bFromSweep :type Boolean) (SweepResult :type Hit%20Result%20Structure%20%28by%20ref%29))
  (Default|SwitchPawntoMiniGame2 (Variables|Default|GetPlayerCharacterREF))
  (Rendering|SetVisibility (Variables|/Game/MiniGame/SwitchPawnLogic/BP_KeyPawn_1.BP_KeyPawn_1_C|GetStaticMesh (Variables|Default|GetKeyPawnRef)) true false))

(event EventBeginPlay
  (bind _returnvalue (Actor|GetActorOfClass "/Game/ThirdPerson/Blueprints/BP_ThirdPersonCharacter.BP_ThirdPersonCharacter_C"))
  (bind _output_get (Variables|Default|SetPlayerCharacterREF _returnvalue))
  (Utilities|IsValid _output_get
    (:Is%20Valid
      (bind _returnvalue_2 (Actor|GetActorOfClass "/Game/MiniGame/SwitchPawnLogic/BP_KeyPawn_1.BP_KeyPawn_1_C"))
      (Variables|Default|SetKeyPawnRef _returnvalue_2))))

(fn ConstructionScript)