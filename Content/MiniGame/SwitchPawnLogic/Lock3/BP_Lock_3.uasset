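; Three-stage lock mini-game that starts on trigger overlap, hiding the player and switching to key pawn C.
; Each key pawn's transform event checks its arrow against the lock's arrow by X/Y position and normalized yaw, within tolerances.
; A match flashes an outline overlay, hides that lock mesh and advances from C to B to A.
; Solving A disables input, stops the audio and opens the win level.
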(event OnComponentBeginOverlap(StartGameBox)
  (params (OverlappedComponent :type Primitive%20Component%20Object%20Reference) (OtherActor :type Actor%20Object%20Reference) (OtherComp :type Primitive%20Component%20Object%20Reference) (OtherBodyIndex :type Integer) (bFromSweep :type Boolean) (SweepResult :type Hit%20Result%20Structure%20%28by%20ref%29))
  (bind _playercharacter_ref (Variables|Default|GetPlayerCharacter_REF))
  (Default|SwitchtoMiniGameC _playercharacter_ref)
  (Rendering|SetActorHiddenInGame _playercharacter_ref true)
  (Rendering|SetVisibility (Variables|/Game/MiniGame/SwitchPawnLogic/Lock3/BP_KeyPawnC.BP_KeyPawnC_C|GetStaticMesh (Variables|Default|GetKeyPawnC_REF)) true false)
  (bind _returnvalue (Utilities|Time|SetTimerbyEvent (delegate Custom|AudioCriss) 2.0 true)))

(event Custom|KeyATransformEvent
  (bind _staticmeshlocka (Variables|Default|GetStaticMeshLockA))
  (bind _match (CallFunction|CompareA))
  (if _match
    (Utilities|ChangeOverlayMaterial _staticmeshlocka)
    (Rendering|SetVisibility _staticmeshlocka false false)
    (Input|DisableInput (Variables|Default|GetKeyPawnA_REF) 0)
    (Utilities|FlowControl|Delay 2.0)
    ;[1 1 1] Open Level Win
    (Game|OpenLevel(byObjectReference) "/Game/Phantasma/Maps/WinLevel.WinLevel")
    (Components|Activation|Deactivate (Variables|Default|GetAudio))
    (Components|Activation|Deactivate (Variables|/Game/Phantasma/Blueprints/BP_Player_Game.BP_Player_Game_C|GetAudio_kitchen (Variables|Default|GetPlayerCharacter_REF)))
    (Utilities|Time|ClearandInvalidateTimerbyHandle (stale OnComponentBeginOverlap(StartGameBox) _returnvalue))))

(event Custom|AudioCriss
  (Components|Activation|Activate (Variables|Default|GetAudio) false))

(event Custom|KeyBTransformEvent
  (bind _keypawna_ref (Variables|Default|GetKeyPawnA_REF))
  (bind _staticmeshb (Variables|Default|GetStaticMeshB))
  (bind _match (CallFunction|CompareB))
  (if _match
    (Utilities|ChangeOverlayMaterial _staticmeshb)
    (Rendering|SetVisibility _staticmeshb false false)
    (Default|SwitchtoMiniGameA (Variables|Default|GetPlayerCharacter_REF))
    (EventDispatchers|BindEventtoOnKeyTransform _keypawna_ref (delegate Custom|KeyATransformEvent))
    (Rendering|SetVisibility (Variables|/Game/MiniGame/SwitchPawnLogic/Lock3/BP_KeyPawnA.BP_KeyPawnA_C|GetStaticMesh _keypawna_ref) true false)))

(event Custom|KeyCTranform
  (bind _staticmeshc (Variables|Default|GetStaticMeshC))
  (bind _keypawnb_ref (Variables|Default|GetKeyPawnB_REF))
  (bind _match (CallFunction|CompareC))
  (if _match
    (Utilities|ChangeOverlayMaterial _staticmeshc)
    (Rendering|SetVisibility _staticmeshc false false)
    (Default|SwitchtoMiniGameB (Variables|Default|GetPlayerCharacter_REF))
    (EventDispatchers|BindEventtoOnKeyTransform _keypawnb_ref (delegate Custom|KeyBTransformEvent))
    (Rendering|SetVisibility (Variables|/Game/MiniGame/SwitchPawnLogic/Lock3/BP_KeyPawnB.BP_KeyPawnB_C|GetStaticMesh _keypawnb_ref) true false)))

(event EventBeginPlay
  (bind _returnvalue (Actor|GetActorOfClass "/Game/Phantasma/Blueprints/BP_Player_Game.BP_Player_Game_C"))
  (bind _output_get (Variables|Default|SetPlayerCharacter_REF _returnvalue))
  (Utilities|IsValid _output_get
    (:Is%20Valid
      (bind _returnvalue_2 (Actor|GetActorOfClass "/Game/MiniGame/SwitchPawnLogic/Lock3/BP_KeyPawnC.BP_KeyPawnC_C"))
      (Variables|Default|SetKeyPawnC_REF _returnvalue_2)
      (bind _returnvalue_3 (Actor|GetActorOfClass "/Game/MiniGame/SwitchPawnLogic/Lock3/BP_KeyPawnB.BP_KeyPawnB_C"))
      (Variables|Default|SetKeyPawnB_REF _returnvalue_3)
      (bind _returnvalue_4 (Actor|GetActorOfClass "/Game/MiniGame/SwitchPawnLogic/Lock3/BP_KeyPawnA.BP_KeyPawnA_C"))
      (Variables|Default|SetKeyPawnA_REF _returnvalue_4)
      (EventDispatchers|BindEventtoOnKeyTransform (Variables|Default|GetKeyPawnC_REF) (delegate Custom|KeyCTranform))
      (Rendering|SetVisibility (Variables|/Game/MiniGame/SwitchPawnLogic/Lock3/BP_KeyPawnC.BP_KeyPawnC_C|GetStaticMesh (Variables|Default|GetKeyPawnC_REF)) true false))))

(fn ConstructionScript)

(fn NormalizeAngle
  (params (Agnle :type Float%20%28double-precision%29))
  (bind _returnvalue (Math|Rotator|NormalizeAxis Agnle))
  (return (Math|Float|SelectFloat _returnvalue (+ _returnvalue 3.6e+02) (>= _returnvalue 0.0))))

(fn CompareA
  (bind _arrowa (Variables|Default|GetArrowA))
  (bind _keypawna_ref (Variables|Default|GetKeyPawnA_REF))
  (bind _returnvalue (Transformation|GetWorldLocation _arrowa))
  (bind _arrowkeya (Variables|/Game/MiniGame/SwitchPawnLogic/Lock3/BP_KeyPawnA.BP_KeyPawnA_C|GetArrowKeyA _keypawna_ref))
  (bind _returnvalue_2 (Transformation|GetWorldLocation _arrowkeya))
  (if (and (Math|Float|NearlyEqual(Float) (.x _returnvalue) (.x _returnvalue_2) 1e+01) (Math|Float|NearlyEqual(Float) (.y _returnvalue) (.y _returnvalue_2) 1e+01))
    (bind _newangle (CallFunction|NormalizeAngle (.yaw (Transformation|GetWorldRotation (Variables|Default|GetArrowA)))))
    (bind _newangle_2 (CallFunction|NormalizeAngle (.yaw (Transformation|GetWorldRotation _arrowkeya))))
    (return (Math|Float|NearlyEqual(Float) _newangle _newangle_2 5.0))))

(fn CompareB
  (bind _keypawnb_ref (Variables|Default|GetKeyPawnB_REF))
  (bind _arrowb (Variables|Default|GetArrowB))
  (bind _returnvalue (Transformation|GetWorldLocation _arrowb))
  (bind _arrowkeyb (Variables|/Game/MiniGame/SwitchPawnLogic/Lock3/BP_KeyPawnB.BP_KeyPawnB_C|GetArrowKeyB _keypawnb_ref))
  (bind _returnvalue_2 (Transformation|GetWorldLocation _arrowkeyb))
  (if (and (Math|Float|NearlyEqual(Float) (.x _returnvalue) (.x _returnvalue_2) 5.0) (Math|Float|NearlyEqual(Float) (.y _returnvalue) (.y _returnvalue_2) 5.0))
    (bind _newangle (CallFunction|NormalizeAngle (.yaw (Transformation|GetWorldRotation (Variables|Default|GetArrowB)))))
    (bind _newangle_2 (CallFunction|NormalizeAngle (.yaw (Transformation|GetWorldRotation _arrowkeyb))))
    (return (Math|Float|NearlyEqual(Float) _newangle _newangle_2 5.0))))

(fn CompareC
  (bind _keypawnc_ref (Variables|Default|GetKeyPawnC_REF))
  (bind _arrowc (Variables|Default|GetArrowC))
  (bind _returnvalue (Transformation|GetWorldLocation _arrowc))
  (bind _arrowkeyc (Variables|/Game/MiniGame/SwitchPawnLogic/Lock3/BP_KeyPawnC.BP_KeyPawnC_C|GetArrowKeyC _keypawnc_ref))
  (bind _returnvalue_2 (Transformation|GetWorldLocation _arrowkeyc))
  (if (and (Math|Float|NearlyEqual(Float) (.x _returnvalue) (.x _returnvalue_2) 5.0) (Math|Float|NearlyEqual(Float) (.y _returnvalue) (.y _returnvalue_2) 5.0))
    (bind _newangle (CallFunction|NormalizeAngle (.yaw (Transformation|GetWorldRotation (Variables|Default|GetArrowC)))))
    (bind _newangle_2 (CallFunction|NormalizeAngle (.yaw (Transformation|GetWorldRotation _arrowkeyc))))
    (return (Math|Float|NearlyEqual(Float) _newangle _newangle_2 5.0))))