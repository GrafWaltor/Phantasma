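; Possessable key pawn for the Lock3 pawn-switching minigame, with its mesh hidden at BeginPlay.
; On possession it adds the player input context and finds FixedCamera_3 by display name, which Tick smoothly turns toward the pawn.
; Enhanced Input drives movement, which fires OnKeyTransform, and yaw rotation, while the up/down action is left empty.
; SwitchToCharacter calls Possess on the player controller and returns the view to BP_Phantasma_Camera.
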(event Input|EnhancedActionEvents|EnhancedInputActionIA_Player_Movement
  (params (ActionValue :type Vector%202D%20Structure) (ElapsedSeconds :type Float%20%28double-precision%29) (TriggeredSeconds :type Float%20%28double-precision%29) (InputAction :type Input%20Action%20Object%20Reference :default "/Game/Phantasma/Blueprints/Inputs/Actions/IA_Player_Movement.IA_Player_Movement"))
  (Pawn|Input|AddMovementInput (* (Math|Vector|GetRightVector (Math|Rotator|MakeRotator 0.0 0.0 0.0)) "-1.000000,-1.000000,-1.000000") (Math|Interpolation|FInterpTo (Variables|Default|GetCurrentValue) (.y ActionValue) (Utilities|Time|GetWorldDeltaSeconds) 1e+01) false)
  (Pawn|Input|AddMovementInput (Math|Vector|GetForwardVector (Math|Rotator|MakeRotator 0.0 (.pitch (Pawn|GetControlRotation :!class /Script/Engine.Pawn)) 0.0)) (Math|Interpolation|FInterpTo (Variables|Default|GetCurrentValue) (.x ActionValue) (Utilities|Time|GetWorldDeltaSeconds) 1e+01) false)
  (Default|CallOnKeyTransform))

(event Input|EnhancedActionEvents|EnhancedInputActionIA_PawnMove_UD
  (params (ActionValue :type Vector :default "0, 0, 0") (ElapsedSeconds :type Float%20%28double-precision%29) (TriggeredSeconds :type Float%20%28double-precision%29) (InputAction :type Input%20Action%20Object%20Reference :default "/Game/ThirdPerson/Input/Actions/IA_PawnMove_UD.IA_PawnMove_UD")))

(event Input|EnhancedActionEvents|EnhancedInputActionIA_RotatePawn
  (params (ActionValue :type Vector :default "0, 0, 0") (ElapsedSeconds :type Float%20%28double-precision%29) (TriggeredSeconds :type Float%20%28double-precision%29) (InputAction :type Input%20Action%20Object%20Reference :default "/Game/Phantasma/Blueprints/Inputs/Actions/IA_RotatePawn.IA_RotatePawn"))
  (Transformation|AddActorLocalRotation (Math|Rotator|MakeRotator 0.0 0.0 (* (.x ActionValue) (Variables|Default|GetRotationSpeed))) false false))

(event EventBeginPlay
  (Rendering|SetVisibility (Variables|Default|GetStaticMesh) false false))

(event EventTick
  (params (DeltaSeconds :type Float%20%28single-precision%29))
  (bind _camera_3 (Variables|Default|GetCamera_3))
  (Utilities|IsValid _camera_3
    (:Is%20Valid
      (Transformation|SetActorRotation _camera_3 (Math|Interpolation|RInterpTo (Transformation|GetActorRotation _camera_3) (Math|Rotator|FindLookatRotation (Transformation|GetActorLocation _camera_3) (Transformation|GetActorLocation)) DeltaSeconds 1.0)))))

(event EventPossessed
  (params (NewController :type Controller%20Object%20Reference))
  (bind _asplayer_controller (Utilities|Casting|CastToPlayerController (Pawn|GetController)))
  (bind _output_get (Variables|Default|SetAs%20Player%20Controller _asplayer_controller))
  (Utilities|IsValid _output_get
    (:Is%20Valid
      (Input|AddMappingContext (PlayerController|LocalPlayerSubsystems|GetEnhancedInputLocalPlayerSubsystem _asplayer_controller) "/Game/Phantasma/Blueprints/Inputs/IMC_Phantasma_PLayer.IMC_Phantasma_PLayer" 0 "(bIgnoreAllPressedKeysUntilRelease=True,bForceImmediately=False,bNotifyUserSettings=False)")
      (bind _outactors (Actor|GetAllActorsOfClass "/Script/Engine.CameraActor"))
      (for _array_element _outactors
        (if (Utilities|Enum|Equal(Enum) (Utilities|GetDisplayName _array_element) "FixedCamera_3")
          (Variables|Default|SetCamera_3 _array_element))))))

(fn ConstructionScript)

(fn SwitchtoCharacter
  (Pawn|Possess (Game|GetPlayerController 0))
  (bind _returnvalue (Actor|GetActorOfClass "/Game/Phantasma/Blueprints/Camera/BP_Phantasma_Camera.BP_Phantasma_Camera_C"))
  (bind _output_get (Variables|Default|SetDefaultCameraREF _returnvalue))
  (Game|Player|SetViewTargetwithBlend (Variables|Default|GetAs%20Player%20Controller) _output_get 0.0 "VTBlend_Linear" 0.0 false))