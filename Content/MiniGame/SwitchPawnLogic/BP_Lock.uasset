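; BP_Lock is the lock in a key-alignment minigame that opens a BP_Hatch.
; Overlapping its start box hides the player, calls the switch to the minigame, reveals the key pawn and starts a looping audio timer.
; Each key transform event compares lock and key arrows by XY position and normalized yaw within tolerances.
; A match flags the hatch's lock open, then after a delay restores the player and destroys key and lock.
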(event OnComponentBeginOverlap(StartGameBox)
  (params (OverlappedComponent :type Primitive%20Component%20Object%20Reference) (OtherActor :type Actor%20Object%20Reference) (OtherComp :type Primitive%20Component%20Object%20Reference) (OtherBodyIndex :type Integer) (bFromSweep :type Boolean) (SweepResult :type Hit%20Result%20Structure%20%28by%20ref%29))
  (bind _playercharacterref (Variables|Default|GetPlayerCharacterREF))
  (Rendering|SetActorHiddenInGame _playercharacterref true)
  (Default|SwitchtoMiniGame1 _playercharacterref)
  (Rendering|SetVisibility (Variables|/Game/MiniGame/SwitchPawnLogic/BP_KeyPawn.BP_KeyPawn_C|GetStaticMesh (Variables|Default|GetKeyPawnRef)) true false)
  (bind _returnvalue (Actor|GetActorOfClass "/Game/Phantasma/Blueprints/Environment/BP_Hatch.BP_Hatch_C"))
  (Variables|Default|SetBP_Hatch _returnvalue)
  (Utilities|Time|SetTimerbyEvent (delegate Custom|AudioCriss) 2.0 true))

(event Custom|OnKeyTransformEvemt
  (bind _keypawnref (Variables|Default|GetKeyPawnRef))
  (bind _match (CallFunction|Compare))
  (if _match
    (Input|DisableInput _keypawnref 0)
    (Rendering|SetVisibility (Variables|/Game/MiniGame/SwitchPawnLogic/BP_KeyPawn.BP_KeyPawn_C|GetStaticMesh _keypawnref) false false)
    (Rendering|Material|SetOverlayMaterial (Variables|Default|GetStaticMesh) "/Game/MiniGame/Materials/Overlay/MI_OutlinesOverlay.MI_OutlinesOverlay" :!class /Script/Engine.MeshComponent)
    (Variables|/Game/Phantasma/Blueprints/Environment/BP_Hatch.BP_Hatch_C|SetbIsLockOpen (Variables|Default|GetBP_Hatch) true)
    (Components|Activation|Activate (Variables|Default|GetAudio) false)
    (Rendering|Material|SetOverlayMaterial (Variables|Default|GetStaticMesh) "/Game/Phantasma/Materials/MI_OverlayOutline.MI_OverlayOutline" :!class /Script/Engine.MeshComponent)
    (Utilities|FlowControl|Delay 3.0)
    (Default|SwitchtoCharacter _keypawnref)
    (Rendering|SetActorHiddenInGame (Variables|Default|GetPlayerCharacterREF) false)
    (Actor|DestroyActor _keypawnref)
    (Actor|DestroyActor)))

(event Custom|AudioCriss
  (Components|Activation|Activate (Variables|Default|GetAudioCris) false))

(event EventBeginPlay
  (bind _returnvalue (Actor|GetActorOfClass "/Game/Phantasma/Blueprints/BP_Player_Game.BP_Player_Game_C"))
  (bind _output_get (Variables|Default|SetPlayerCharacterREF _returnvalue))
  (Utilities|IsValid _output_get
    (:Is%20Valid
      (bind _returnvalue_2 (Actor|GetActorOfClass "/Game/MiniGame/SwitchPawnLogic/BP_KeyPawn.BP_KeyPawn_C"))
      (Variables|Default|SetKeyPawnRef _returnvalue_2)
      (EventDispatchers|BindEventtoOnKeyTransform (Variables|Default|GetKeyPawnRef) (delegate Custom|OnKeyTransformEvemt)))))

(fn ConstructionScript)

(fn NormalizeAngle
  (params (Agnle :type Float%20%28double-precision%29))
  (bind _returnvalue (Math|Rotator|NormalizeAxis Agnle))
  (return (Math|Float|SelectFloat _returnvalue (+ _returnvalue 3.6e+02) (>= _returnvalue 0.0))))

(fn Compare
  (bind _keypawnref (Variables|Default|GetKeyPawnRef))
  (bind _lockarrow (Variables|Default|GetLockArrow))
  (bind _returnvalue (Transformation|GetWorldLocation _lockarrow))
  (bind _arrow (Variables|/Game/MiniGame/SwitchPawnLogic/BP_KeyPawn.BP_KeyPawn_C|GetArrow _keypawnref))
  (bind _returnvalue_2 (Transformation|GetWorldLocation _arrow))
  (if (and (Math|Float|NearlyEqual(Float) (.x _returnvalue) (.x _returnvalue_2) 5.0) (Math|Float|NearlyEqual(Float) (.y _returnvalue) (.y _returnvalue_2) 5.0))
    (bind _newangle (CallFunction|NormalizeAngle (.yaw (Transformation|GetWorldRotation (Variables|Default|GetLockArrow)))))
    (bind _newangle_2 (CallFunction|NormalizeAngle (.yaw (Transformation|GetWorldRotation (Variables|/Game/MiniGame/SwitchPawnLogic/BP_KeyPawn.BP_KeyPawn_C|GetArrow (Variables|Default|GetKeyPawnRef))))))
    (return (Math|Float|NearlyEqual(Float) _newangle _newangle_2 2.0))))