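; BP_KeyPawn is the possessable key pawn for a minigame, with its mesh hidden at BeginPlay.
; On possession it adds the input mapping and caches the player character and minigame camera, which Tick smoothly rotates toward the pawn.
; Enhanced Input moves and yaws the pawn, firing OnKeyTransform on each input.
; SwitchToCharacter repossesses the player character and blends the view back to the Phantasma camera.
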(event Input|EnhancedActionEvents|EnhancedInputActionIA_Player_Movement
  (params (ActionValue :type Vector%202D%20Structure) (ElapsedSeconds :type Float%20%28double-precision%29) (TriggeredSeconds :type Float%20%28double-precision%29) (InputAction :type Input%20Action%20Object%20Reference :default "/Game/Phantasma/Blueprints/Inputs/Actions/IA_Player_Movement.IA_Player_Movement"))
  (Pawn|Input|AddMovementInput (Math|Vector|GetRightVector (Math|Rotator|MakeRotator 0.0 0.0 0.0)) (Math|Interpolation|FInterpTo (Variables|Default|GetCurrentValue) (.y ActionValue) (Utilities|Time|GetWorldDeltaSeconds) 1e+01) false)
  (Pawn|Input|AddMovementInput (* (Math|Vector|GetForwardVector (Math|Rotator|MakeRotator 0.0 (.pitch (Pawn|GetControlRotation :!class /Script/Engine.Pawn)) 0.0)) "-1.000000,0.000000,0.000000") (Math|Interpolation|FInterpTo (Variables|Default|GetCurrentValue) (.x ActionValue) (Utilities|Time|GetWorldDeltaSeconds) 1e+01) false)
  (Default|CallOnKeyTransform))

(event Input|EnhancedActionEvents|EnhancedInputActionIA_RotatePawn
  (params (ActionValue :type Vector :default "0, 0, 0") (ElapsedSeconds :type Float%20%28double-precision%29) (TriggeredSeconds :type Float%20%28double-precision%29) (InputAction :type Input%20Action%20Object%20Reference :default "/Game/Phantasma/Blueprints/Inputs/Actions/IA_RotatePawn.IA_RotatePawn"))
  (Transformation|AddActorLocalRotation (Math|Rotator|MakeRotator 0.0 0.0 (* (.x ActionValue) (Variables|Default|GetRotationSpeed))) false false)
  (Default|CallOnKeyTransform))

(event EventBeginPlay
  (Rendering|SetVisibility (Variables|Default|GetStaticMesh) false false))

(event EventTick
  (params (DeltaSeconds :type Float%20%28single-precision%29))
  (bind _bp_cametaref (Variables|Default|GetBP_CametaREF))
  (Utilities|IsValid _bp_cametaref
    (:Is%20Valid
      (Transformation|SetActorRotation _bp_cametaref (Math|Interpolation|RInterpTo (Transformation|GetActorRotation _bp_cametaref) (Math|Rotator|FindLookatRotation (Transformation|GetActorLocation _bp_cametaref) (Transformation|GetActorLocation)) DeltaSeconds 1.0)))))

(event EventPossessed
  (params (NewController :type Controller%20Object%20Reference))
  (bind _asplayer_controller (Utilities|Casting|CastToPlayerController (Pawn|GetController)))
  (Utilities|IsValid (PlayerController|LocalPlayerSubsystems|GetEnhancedInputLocalPlayerSubsystem _asplayer_controller)
    (:Is%20Valid
      (Input|AddMappingContext (PlayerController|LocalPlayerSubsystems|GetEnhancedInputLocalPlayerSubsystem _asplayer_controller) "/Game/Phantasma/Blueprints/Inputs/IMC_Phantasma_PLayer.IMC_Phantasma_PLayer" 0 "(bIgnoreAllPressedKeysUntilRelease=True,bForceImmediately=False,bNotifyUserSettings=False)")
      (bind _returnvalue (Actor|GetActorOfClass "/Game/Phantasma/Blueprints/BP_Player_Game.BP_Player_Game_C"))
      (Variables|Default|SetPlayerCharacterRef _returnvalue)
      (bind _returnvalue_2 (Actor|GetActorOfClass "/Game/Phantasma/Blueprints/Camera/BP_MiniGameCamera.BP_MiniGameCamera_C"))
      (Variables|Default|SetBP_CametaREF _returnvalue_2))))

(fn ConstructionScript)

(fn SwitchtoCharacter
  (bind _returnvalue (Game|GetPlayerController 0))
  (Pawn|Possess _returnvalue (Variables|Default|GetPlayerCharacterRef))
  (bind _returnvalue_2 (Actor|GetActorOfClass "/Game/Phantasma/Blueprints/Camera/BP_Phantasma_Camera.BP_Phantasma_Camera_C"))
  (bind _output_get (Variables|Default|SetDefaultCameraREF _returnvalue_2))
  (Game|Player|SetViewTargetwithBlend _returnvalue _output_get 3.0 "VTBlend_Linear" 0.0 false))