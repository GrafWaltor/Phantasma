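; BP_Pillow is a pillow Blueprint that runs a countdown ending in the player's death.
; Pillow_Event starts a looping one-second timer that decrements MaxTime and copies the result to PillowTime.
; Each tick prints debug warnings for every threshold the remaining time has reached.
; At zero it clears the timer, casts the player pawn to BP_Player_Game and calls Death.
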(event Custom|Pillow_Event
  (bind _returnvalue (Utilities|Time|SetTimerbyEvent (delegate Custom|CustomEvent) 1.0 true))
  (bind _output_get (Variables|Default|SetTimer_Pillow _returnvalue)))

(event Custom|CustomEvent
  (bind _result (Math|Float|DecrementFloat (Variables|Default|GetMaxTime))
    (:%20%20
      (bind _output_get (Variables|Default|SetPillow_time _result))
      (Utilities|FlowControl|Sequence
        (:then_0
          (if (<= _output_get 15.0)
            (Development|PrintString "15")))
        (:then_1
          (if (<= _output_get 1e+01)
            (Development|PrintString "10")))
        (:then_2
          (if (<= _output_get 5.0)
            (Development|PrintString "5")))
        (:then_3
          (if (<= _output_get 0.0)
            (Utilities|Time|ClearandInvalidateTimerbyHandle (stale Custom|Pillow_Event _output_get))
            (bind _asbp_player_game (Utilities|Casting|CastToBP_Player_Game (Game|Player|GetPlayerPawn 0)))
            (Default|Death _asbp_player_game)))))))

(event EventBeginPlay)

(event Collision|EventActorBeginOverlap
  (params (OtherActor :type Actor%20Object%20Reference)))

(event EventTick
  (params (DeltaSeconds :type Float%20%28single-precision%29)))

(fn ConstructionScript)