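; BP_Eye is an environment eye actor that smoothly turns to watch the player character.
; On BeginPlay it caches BP_Player_Game and, if valid, plays the EyeRotation timeline to drive the Arrow component's relative yaw.
; Each Tick it interpolates the whole actor's rotation toward a look-at from the Arrow's location to the player, without rechecking that the cached reference is valid.
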(event EventBeginPlay
  (bind _returnvalue (Actor|GetActorOfClass "/Game/Phantasma/Blueprints/BP_Player_Game.BP_Player_Game_C"))
  (bind _output_get (Variables|Default|SetPlayerCharacter_REF _returnvalue))
  (Utilities|IsValid _output_get
    (:Is%20Valid
      (bind _rotation (Timeline|EyeRotation Play)
        (:Update
          (Transformation|SetRelativeRotation (Variables|Default|GetArrow) (Math|Rotator|MakeRotator 0.0 0.0 _rotation) false false))))))

(event EventTick
  (params (DeltaSeconds :type Float%20%28single-precision%29))
  (Transformation|SetActorRotation (Math|Interpolation|RInterpTo (Transformation|GetActorRotation) (Math|Rotator|FindLookatRotation (Transformation|GetWorldLocation (Variables|Default|GetArrow)) (Transformation|GetActorLocation (Variables|Default|GetPlayerCharacter_REF))) (Utilities|Time|GetWorldDeltaSeconds) 2.0)))

(fn ConstructionScript)