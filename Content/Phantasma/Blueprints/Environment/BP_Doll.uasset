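; BP_Doll is an environment doll prop in Phantasma that plays a sitting animation and then releases an AI_Hands actor.
; The RunSitingAnimation event drives a timeline that sets the root's pitch to tilt the doll.
; When the timeline finishes, it destroys the head and both hand components and spawns AI_Hands at the doll's transform.
; BeginPlay, Tick and SitFunc are empty.
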(event Custom|RunSitingAnimation
  (bind _roottrack (Timeline|SittingAnimation Play)
    (:Update
      (Transformation|SetWorldRotation (Variables|Default|GetRoot) (Math|Rotator|MakeRotator 0.0 _roottrack 0.0) false false))
    (:Finished
      (Components|DestroyComponent (Variables|Default|GetHead))
      (Components|DestroyComponent (Variables|Default|GetHand_R))
      (Components|DestroyComponent (Variables|Default|GetHand_L))
      (Game|SpawnActorfromClass "/Game/Phantasma/EnemyGame/AI/AI_BP/AI_Hands.AI_Hands_C" (Transformation|GetActorTransform self) "Undefined" "MultiplyWithRoot" 0 0 0))))

(event EventBeginPlay)

(event Collision|EventActorBeginOverlap
  (params (OtherActor :type Actor%20Object%20Reference)))

(event EventTick
  (params (DeltaSeconds :type Float%20%28single-precision%29)))

(fn ConstructionScript)

(fn SitFunc)