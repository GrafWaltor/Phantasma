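; BP_DollHands is an environment doll actor that plays a start animation, then travels along a spline path.
; On BeginPlay it finds the BP_SplineDollPath actor, then a timeline yaws and raises or lowers the head and slides both hand roots sideways to detach them.
; When that finishes, a second timeline, rate-scaled by TimeToComplite, moves the actor along the spline's length, following location only.
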(event EventBeginPlay
  (bind _returnvalue (Actor|GetActorOfClass "/Game/Phantasma/Blueprints/Environment/BP_SplineDollPath.BP_SplineDollPath_C"))
  (Variables|Default|SetSplinePath _returnvalue)
  (bind (_direction _headrotation _headlocation _lefthanddeattach _righthanddeattach) (Timeline|StartAnimation Play)
    (:Update
      (Transformation|SetWorldRotation (Variables|Default|GetArrowHead) (Math|Rotator|MakeRotator 0.0 0.0 _headrotation) false false)
      (Transformation|SetRelativeLocation (Variables|Default|GetArrowHead) (Math|Vector|MakeVector 0.0 0.0 _headlocation) false false)
      (Transformation|SetRelativeLocation (Variables|Default|GetRoot_Hand_L) (Math|Vector|MakeVector 4.98606 _lefthanddeattach 18.266667) false false)
      (Transformation|SetRelativeLocation (Variables|Default|GetRoot_Hand_R) (Math|Vector|MakeVector 4.98606 _righthanddeattach 18.266667) false false))
    (:Finished
      (Components|Timeline|SetPlayRate (Variables|Default|GetSpline_Timeline) (/ 1.0 (Variables|Default|GetTimeToComplite)))
      (bind _newtrack_1 (Timeline|Spline_Timeline Play)
        (:Update
          (Transformation|SetActorTransform (Math|Transform|MakeTransform (Spline|GetLocationatDistanceAlongSpline (Variables|/Game/Phantasma/Blueprints/Environment/BP_SplineDollPath.BP_SplineDollPath_C|GetSpline (Variables|Default|GetSplinePath)) (Math|Float|Lerp 0.0 (Spline|GetSplineLength (Variables|/Game/Phantasma/Blueprints/Environment/BP_SplineDollPath.BP_SplineDollPath_C|GetSpline (Variables|Default|GetSplinePath))) _newtrack_1) "World") "0, 0, 0" (Transformation|GetActorScale3D))))))))

(event Collision|EventActorBeginOverlap
  (params (OtherActor :type Actor%20Object%20Reference)))

(fn ConstructionScript)

(fn SitFunc)