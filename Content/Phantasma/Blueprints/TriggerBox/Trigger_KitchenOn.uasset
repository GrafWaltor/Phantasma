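; Trigger box that switches on the kitchen sequence when the player enters it.
; On box overlap by BP_Player_Game, it activates the player's AudioKitchen component and plays the PhaseOneBGREF and ChristopgerKitchen references from the start.
; It also finds AI_BukaController and sets it to its passive state.
; Nothing disables the trigger, so every new player overlap runs the sequence again.
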(event OnComponentBeginOverlap(Box)
  (params (OverlappedComponent :type Primitive%20Component%20Object%20Reference) (OtherActor :type Actor%20Object%20Reference) (OtherComp :type Primitive%20Component%20Object%20Reference) (OtherBodyIndex :type Integer) (bFromSweep :type Boolean) (SweepResult :type Hit%20Result%20Structure%20%28by%20ref%29))
  (bind _asbp_player_game (Utilities|Casting|CastToBP_Player_Game (Game|Player|GetPlayerPawn 0)))
  (if (== _asbp_player_game OtherActor)
    (Components|Activation|Activate (Variables|/Game/Phantasma/Blueprints/BP_Player_Game.BP_Player_Game_C|GetAudio_kitchen _asbp_player_game) false)
    (bind _returnvalue (Actor|GetActorOfClass "/Game/Phantasma/EnemyGame/AI/AI_BukaController.AI_BukaController_C"))
    (bind _output_get (Variables|Default|SetBukaController _returnvalue))
    (Default|SetPassiveState _output_get)
    (Audio|Components|Audio|Play (Variables|Default|GetPhaseOneBG_REF) 0.0)
    (Audio|Components|Audio|Play (Variables|Default|GetChristopger_Kitchen) 0.0)))

(event EventBeginPlay)

(event Collision|EventActorBeginOverlap
  (params (OtherActor :type Actor%20Object%20Reference)))

(event EventTick
  (params (DeltaSeconds :type Float%20%28single-precision%29)))

(fn ConstructionScript)