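; Trigger volume that pacifies the Buka AI when the player enters it.
; On BeginPlay it caches the AI_BukaController found in the level through GetActorOfClass.
; When the BP_Player_Game character overlaps the Box, it turns off that controller's PawnSensing updates and calls SetPassiveState.
; Nothing in this Blueprint re-enables sensing afterwards.
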(event OnComponentBeginOverlap(Box)
  (params (OverlappedComponent :type Primitive%20Component%20Object%20Reference) (OtherActor :type Actor%20Object%20Reference) (OtherComp :type Primitive%20Component%20Object%20Reference) (OtherBodyIndex :type Integer) (bFromSweep :type Boolean) (SweepResult :type Hit%20Result%20Structure%20%28by%20ref%29))
  (bind _ai_controller (Variables|Default|GetAI_Controller))
  (bind _asbp_player_game (Utilities|Casting|CastToBP_Player_Game (Game|GetPlayerCharacter 0)))
  (Utilities|IsValid _asbp_player_game
    (:Is%20Valid
      (if (== OtherActor _asbp_player_game)
        (Class|PawnSensingComponent|SetSensingUpdatesEnabled (Variables|/Game/Phantasma/EnemyGame/AI/AI_BukaController.AI_BukaController_C|GetPawnSensing _ai_controller) false)
        (Default|SetPassiveState _ai_controller)))))

(event EventBeginPlay
  (bind _returnvalue (Actor|GetActorOfClass "/Game/Phantasma/EnemyGame/AI/AI_BukaController.AI_BukaController_C"))
  (Variables|Default|SetAI_Controller _returnvalue))

(event Collision|EventActorBeginOverlap
  (params (OtherActor :type Actor%20Object%20Reference)))

(event EventTick
  (params (DeltaSeconds :type Float%20%28single-precision%29)))

(fn ConstructionScript)