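; Trigger volume that applies camera shake and a post-process effect while the player is inside, apparently for a basement ("Podval") area.
; When the player pawn enters the Box, it calls CamShake on BP_Player_Game and enables the PostProcess component.
; On exit, it clears the player's TimerShake timer and disables the PostProcess.
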(event OnComponentBeginOverlap(Box)
  (params (OverlappedComponent :type Primitive%20Component%20Object%20Reference) (OtherActor :type Actor%20Object%20Reference) (OtherComp :type Primitive%20Component%20Object%20Reference) (OtherBodyIndex :type Integer) (bFromSweep :type Boolean) (SweepResult :type Hit%20Result%20Structure%20%28by%20ref%29))
  (bind _asbp_player_game (Utilities|Casting|CastToBP_Player_Game (Game|Player|GetPlayerPawn 0)))
  (if (== _asbp_player_game OtherActor)
    (Default|CamShake _asbp_player_game)
    (Variables|/Script/Engine.PostProcessComponent|SetbEnabled (Variables|Default|GetPostProcess) true)))

(event OnComponentEndOverlap(Box)
  (params (OverlappedComponent :type Primitive%20Component%20Object%20Reference) (OtherActor :type Actor%20Object%20Reference) (OtherComp :type Primitive%20Component%20Object%20Reference) (OtherBodyIndex :type Integer))
  (bind _asbp_player_game (Utilities|Casting|CastToBP_Player_Game (Game|Player|GetPlayerPawn 0)))
  (if (== OtherActor _asbp_player_game)
    (Utilities|Time|ClearandInvalidateTimerbyHandle (Variables|/Game/Phantasma/Blueprints/BP_Player_Game.BP_Player_Game_C|GetTimer_Shake _asbp_player_game))
    (Variables|/Script/Engine.PostProcessComponent|SetbEnabled (Variables|Default|GetPostProcess) false)))

(event EventBeginPlay)

(event Collision|EventActorBeginOverlap
  (params (OtherActor :type Actor%20Object%20Reference)))

(event EventTick
  (params (DeltaSeconds :type Float%20%28single-precision%29)))

(fn ConstructionScript)