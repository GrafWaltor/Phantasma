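; CrounchTrigger is a trigger actor that kills the player on entering its Box unless the player's IsPillowHead flag is set.
; It caches the BP_Player_Game pawn on BeginPlay and checks its Crouch state every Tick.
; Crouching disables collision on a separate Box1, with no re-enable in this Blueprint.
; Overlap events also track IsCharacterInBox for any actor, but that flag drives no behavior.
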(event OnComponentBeginOverlap(Box)
  (params (OverlappedComponent :type Primitive%20Component%20Object%20Reference) (OtherActor :type Actor%20Object%20Reference) (OtherComp :type Primitive%20Component%20Object%20Reference) (OtherBodyIndex :type Integer) (bFromSweep :type Boolean) (SweepResult :type Hit%20Result%20Structure%20%28by%20ref%29))
  (bind _playercharacter_ref (Variables|Default|GetPlayerCharacter_REF))
  (Variables|Default|SetbIsCharacterInBox true)
  (if (== OtherActor _playercharacter_ref)
    (if (not (Variables|/Game/Phantasma/Blueprints/BP_Player_Game.BP_Player_Game_C|GetIsPillowHead _playercharacter_ref))
      (Default|Death _playercharacter_ref))))

(event OnComponentEndOverlap(Box)
  (params (OverlappedComponent :type Primitive%20Component%20Object%20Reference) (OtherActor :type Actor%20Object%20Reference) (OtherComp :type Primitive%20Component%20Object%20Reference) (OtherBodyIndex :type Integer))
  (Variables|Default|SetbIsCharacterInBox false))

(event EventBeginPlay
  (bind _asbp_player_game (Utilities|Casting|CastToBP_Player_Game (Game|Player|GetPlayerPawn 0)))
  (Variables|Default|SetPlayerCharacter_REF _asbp_player_game))

(event EventTick
  (params (DeltaSeconds :type Float%20%28single-precision%29))
  (if (Variables|/Game/Phantasma/Blueprints/BP_Player_Game.BP_Player_Game_C|GetCrouch? (Variables|Default|GetPlayerCharacter_REF))
    (Collision|SetCollisionEnabled (Variables|Default|GetBox1) "NoCollision")
    (if (Variables|Default|GetbIsCharacterInBox)
      _)))

(fn ConstructionScript)